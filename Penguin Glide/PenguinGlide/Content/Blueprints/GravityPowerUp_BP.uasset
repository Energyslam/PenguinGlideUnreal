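; Gravity power-up actor that, despite its name, provides a MakeDark effect that temporarily dims the level's sun.
; On BeginPlay it enlarges itself and caches the first SunCycle actor; its construction script turns off mesh gravity and linear damping.
; MakeDark lowers that light's intensity, plays the GravityNormal sound and sets a by-name timer for MakeLight on the SunCycle.
; Nothing here calls MakeDark, as the overlap event is disabled.
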(event Custom|MakeDark
  (Rendering|Components|Light|SetIntensity (Variables|/Script/Engine.Light|GetLightComponent (stale EventBeginPlay _output_get)) (Math|Conversions|ToFloat(Integer) 1))
  (Audio|PlaySound2D "/Game/Audio/GravityNormal.GravityNormal" 1.0 1.0 0.0 0 0)
  (Utilities|Time|SetTimerbyFunctionName (Utilities|Array|Get(acopy) (stale EventBeginPlay _outactors)) "MakeLight" 9.0))

(event EventBeginPlay
  (Transformation|SetActorScale3D "1.200000,1.200000,1.200000")
  (bind _outactors (Actor|GetAllActorsOfClass "/Game/Blueprints/SunCycle.SunCycle_C"))
  (bind _output_get (Variables|Default|SetLightComponent (Utilities|Array|Get(acopy) _outactors))))

(event Collision|EventActorBeginOverlap
  (params (OtherActor :type Actor%20Object%20Reference)))

(event EventTick
  (params (DeltaSeconds :type Float%20%28single-precision%29)))

(fn ConstructionScript
  (Class|PrimitiveComponent|SetLinearDamping (Variables|Default|GetStaticMesh) 0.0)
  (Physics|SetEnableGravity (Variables|Default|GetStaticMesh) false))