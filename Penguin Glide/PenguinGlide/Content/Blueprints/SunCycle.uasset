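; SunCycle controls the intensity of a referenced light and keeps a sky sphere updated.
; BeginPlay randomly sets the light intensity to either negative one or zero, and Tick refreshes the SkySphere material every frame.
; MakeLight forces the negative intensity and plays the GravityReverse 2D sound, with no caller in this Blueprint.
; Despite the name, nothing here rotates the light or advances time.
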(event EventBeginPlay
  (Rendering|Components|Light|SetIntensity (Variables|/Script/Engine.Light|GetLightComponent (Variables|Default|GetLight)) (Math|Conversions|ToFloat(Integer) (Math|Random|RandomIntegerinRange -1 0))))

(event EventTick
  (params (DeltaSeconds :type Float%20%28single-precision%29))
  (Default|RefreshMaterial (Variables|Default|GetSkySphere)))

(fn ConstructionScript)

(fn MakeLight
  (Rendering|Components|Light|SetIntensity (Variables|/Script/Engine.Light|GetLightComponent (Variables|Default|GetLight)) (Math|Conversions|ToFloat(Integer) -1))
  (Audio|PlaySound2D "/Game/Audio/GravityReverse.GravityReverse" 1.0 1.0 0.0 0 0))