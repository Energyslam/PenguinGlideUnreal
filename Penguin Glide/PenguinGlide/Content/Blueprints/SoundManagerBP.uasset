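; SoundManagerBP is an actor that serves as a central trigger point for gameplay sound effects, covering cues such as impacts, pickups-style score bonuses, speed boosts and gravity changes.
; Each custom event plays one fixed sound non-spatially through PlaySound2D, with no state or shared logic.
; A separate StartFadeOut event creates and plays the BlackToFade level sequence for a screen fade.
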(event Custom|PlayImpactSound
  (Audio|PlaySound2D "/Game/Audio/ImpactWAV.ImpactWAV" 1.0 1.0 0.0 0 0))

(event Custom|StartFadeOut
  (bind _outactor (Sequencer|Player|CreateLevelSequencePlayer "/Game/Sequence/BlackToFade.BlackToFade"))
  (Sequencer|Player|Play (Variables|/Script/LevelSequence.LevelSequenceActor|GetSequencePlayer _outactor) :!class /Script/MovieScene.MovieSceneSequencePlayer))

(event Custom|PlayMultiplier
  (Audio|PlaySound2D "/Game/Audio/Multiplier.Multiplier" 1.0 1.0 0.0 0 0))

(event Custom|PlayInstantPoints
  (Audio|PlaySound2D "/Game/Audio/InstantPoints.InstantPoints" 1.0 1.0 0.0 0 0))

(event Custom|PlayWahh
  (Audio|PlaySound2D "/Game/Audio/wahhhh.wahhhh" 1.0 1.0 0.0 0 0))

(event Custom|PlaySpeedUpSound
  (Audio|PlaySound2D "/Game/Audio/SpeedBoostSound.SpeedBoostSound" 1.0 1.0 0.0 0 0))

(event Custom|PlayShake
  (Audio|PlaySound2D "/Game/Audio/shake.shake" 1.0 1.0 0.0 0 0))

(event Custom|PlayGravityDown
  (Audio|PlaySound2D "/Game/Audio/GravityReverse.GravityReverse" 1.0 1.0 0.0 0 0))

(event Custom|PlayGravityUp
  (Audio|PlaySound2D "/Game/Audio/GravityNormal.GravityNormal" 1.0 1.0 0.0 0 0))

(event Custom|PlayIcecrack
  (Audio|PlaySound2D "/Game/Audio/IceCrack.IceCrack" 1.0 1.0 0.0 0 0))

(event EventBeginPlay)

(event Collision|EventActorBeginOverlap
  (params (OtherActor :type Actor%20Object%20Reference)))

(event EventTick
  (params (DeltaSeconds :type Float%20%28single-precision%29)))

(fn ConstructionScript)